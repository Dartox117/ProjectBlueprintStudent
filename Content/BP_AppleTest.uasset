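; BP_AppleTest is a test actor, named as an apple, that bounces and grows on hard vertical impacts.
; When a StaticMesh hit has a high enough upward normal impulse, it applies Force along Z to the mesh.
; Each such hit then reduces Force geometrically and enlarges the actor's scale by a fixed step until its X scale exceeds a limit.
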(event OnComponentHit(StaticMesh)
  (params (HitComponent :type Primitive%20Component%20Object%20Reference) (OtherActor :type Actor%20Object%20Reference) (OtherComp :type Primitive%20Component%20Object%20Reference) (NormalImpulse :type Vector :default "0, 0, 0") (Hit :type Hit%20Result%20Structure%20%28by%20ref%29))
  (bind _returnvalue (Transformation|GetActorScale3D))
  (if (>= (.z NormalImpulse) 1e+03)
    (Physics|AddForce (Variables|Default|GetStaticMesh) (Math|Vector|MakeVector 0.0 0.0 (Variables|Default|GetForce)) "None" false)
    (Variables|Default|SetForce (/ (Variables|Default|GetForce) 1.2))
    (if (not (> (.x _returnvalue) 3.0))
      (Transformation|SetActorScale3D (+ (Math|Vector|MakeVector (.x _returnvalue) (.y _returnvalue) (.z _returnvalue)) "0.500000,0.500000,0.500000")))))

(fn ConstructionScript)