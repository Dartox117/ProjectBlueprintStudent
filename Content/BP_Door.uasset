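; Double door Blueprint that swings two mesh leaves open or closed in opposite directions.
; Each OpenDoor call flips IsClosed and plays or reverses the RotationDoor timeline, which drives the leaves' relative yaw by RotationAngle, with the second leaf offset by a half turn.
; The construction script poses both leaves from IsClosed and sets the timeline time to match the starting state.
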(event Custom|OpenDoor
  (if (Variables|Default|GetIsClosed)
    (Variables|Default|SetIsClosed false)
    (bind _rotationvalue (Timeline|RotationDoor Play)
      (:Update
        (Transformation|SetRelativeRotation (Variables|Default|GetDoor_3_StaticMeshComponent0) (Math|Rotator|MakeRotator 0.0 0.0 (* _rotationvalue -1.0 (Variables|Default|GetRotationAngle))) false false)
        (Transformation|SetRelativeRotation (Variables|Default|GetDoor_4_StaticMeshComponent0) (Math|Rotator|MakeRotator 0.0 0.0 (Math|Float|Lerp 1.8e+02 (+ (Variables|Default|GetRotationAngle) 1.8e+02) _rotationvalue)) false false)))
    (else
      (Variables|Default|SetIsClosed true)
      (Timeline|RotationDoor Reverse))))

(fn ConstructionScript
  (Transformation|SetRelativeRotation (Variables|Default|GetDoor_3_StaticMeshComponent0) (Math|Rotator|MakeRotator 0.0 0.0 (select (Variables|Default|GetIsClosed) 0.0 (* (Variables|Default|GetRotationAngle) -1.0))) false false)
  (Transformation|SetRelativeRotation (Variables|Default|GetDoor_4_StaticMeshComponent0) (Math|Rotator|MakeRotator 0.0 0.0 (select (Variables|Default|GetIsClosed) 1.8e+02 (+ (Variables|Default|GetRotationAngle) 1.8e+02))) false false)
  (Components|Timeline|SetNewTime (Variables|Default|GetRotationDoor) (select (Variables|Default|GetIsClosed) 0.0 1.0)))