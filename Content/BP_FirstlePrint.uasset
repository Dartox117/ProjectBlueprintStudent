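; BP_FirstlePrint is an actor that plays an impact sound when its static mesh takes a strong enough hit.
; The component hit event compares the vertical (Z) normal impulse against the Force threshold.
; A qualifying hit usually plays a falling-object sound at the mesh's location, with a one-in-five random chance of playing a recorded clip instead.
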(event OnComponentHit(StaticMesh)
  (params (HitComponent :type Primitive%20Component%20Object%20Reference) (OtherActor :type Actor%20Object%20Reference) (OtherComp :type Primitive%20Component%20Object%20Reference) (NormalImpulse :type Vector :default "0, 0, 0") (Hit :type Hit%20Result%20Structure%20%28by%20ref%29))
  (if (>= (.z NormalImpulse) (Variables|Default|GetForce))
    (if (== (Math|Random|RandomInteger 5) 4)
      (Audio|PlaySoundatLocation "/Game/Record__online-voice-recorder_com_.Record__online-voice-recorder_com_" (Transformation|GetWorldLocation (Variables|Default|GetStaticMesh)) "0, 0, 0" 1.0 1.0 0.0 0 0 0 0)
      (else
        (Audio|PlaySoundatLocation "/Game/86890__icaroferre__objectfalling1.86890__icaroferre__objectfalling1" (Transformation|GetWorldLocation (Variables|Default|GetStaticMesh)) "0, 0, 0" 1.0 1.0 0.0 0 0 0 0)))))

(event EventBeginPlay)

(event EventTick
  (params (DeltaSeconds :type Float%20%28single-precision%29)))

(fn ConstructionScript)